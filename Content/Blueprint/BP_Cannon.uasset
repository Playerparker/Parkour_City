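; BP_Cannon is a cannon actor that fires a BP_Cannonball whenever another actor begins overlapping it.
; The overlap spawns the ball at the Spawn component's transform and adds acceleration-based force along its Ammo component's forward vector.
; That force is the unscaled unit vector, as the multiplication by Force is left unconnected.
; The LaunchCannonball event only prints debug text.
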(event Custom|Launch%20Cannonball
  (Development|PrintText "LAUNCH CANNNON"))

(event Collision|EventActorBeginOverlap
  (params (OtherActor :type Actor%20Object%20Reference))
  (CallFunction|LaunchCannonball)
  (bind _returnvalue (Game|SpawnActorfromClass "/Game/Blueprint/BP_Cannonball.BP_Cannonball_C" (Transformation|GetWorldTransform (Variables|Components|GetSpawn)) "Undefined" "MultiplyWithRoot" 0 0))
  (Physics|AddForce (Variables|/Game/Blueprint/BP_Cannonball.BP_Cannonball_C|GetAmmo _returnvalue) (Math|Vector|GetForwardVector (Variables|/Game/Blueprint/BP_Cannonball.BP_Cannonball_C|GetAmmo _returnvalue)) "None" true)
  (Development|PrintText "POWWER"))

(fn ConstructionScript)