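; BP_DialogMan is a dialogue manager Blueprint that shows one line from its Dialouge array per DisplayNextLine call.
; It creates a W_DIAL widget on BeginPlay for reuse by every line.
; DisplayNextLine wraps the index at the array's end, prints the line, calls ShowUI, then advances.
; ShowUI sets the widget's text, adds it to the viewport and removes it after a fixed delay.
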(event Custom|DisplayNextLine
  (if (>= (Variables|Default|GetIndex) (Utilities|Array|Length (Variables|Default|GetDialouge)))
    (Variables|Default|SetIndex 0))
  (Development|PrintText (Utilities|Array|Get(acopy) (Variables|Default|GetDialouge) (Variables|Default|GetIndex)) true true "(R=0.000000,G=0.660000,B=1.000000,A=1.000000)" 5.0)
  (CallFunction|ShowUI)
  (Math|Integer|IncrementInt (Variables|Default|GetIndex)))

(event Custom|ShowUI
  (bind _widget (Variables|Default|GetWidget))
  (Rendering|Components|TextRender|SetText (Variables|/Game/Widgets/W_DIAL.W_DIAL_C|GetTextBlock_0 (Variables|Default|GetWidget)) (Utilities|Array|Get(acopy) (Variables|Default|GetDialouge) (Variables|Default|GetIndex)))
  (UserInterface|Viewport|AddtoViewport _widget 0)
  (Utilities|FlowControl|Delay 5.0)
  (Widget|RemovefromParent _widget))

(event EventBeginPlay
  (bind _returnvalue (UserInterface|CreateWidget "/Game/Widgets/W_DIAL.W_DIAL_C"))
  (Variables|Default|SetWidget _returnvalue))

(fn ConstructionScript)