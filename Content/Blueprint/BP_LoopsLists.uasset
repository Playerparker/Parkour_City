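; Loops and lists practice Blueprint that periodically gathers every BP_Tree actor, aiming to nudge each along X, and prints their count as "raised".
; MakeTreesMove starts shortly after BeginPlay and re-calls itself after a delay.
; A Delay inside the for-each does not pause iteration, so only the last tree moves per pass.
; An unconnected while-loop countdown printing in cycling colours never runs.
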(event Custom|MakeTreesMove
  ;[0.15 0.15 0.15 0.5] Comment
  (bind _outactors (Actor|GetAllActorsOfClass "/Game/Blueprint/BP_Tree.BP_Tree_C"))
  (for _array_element _outactors
    (Utilities|FlowControl|Delay 5.0)
    (Transformation|AddRelativeLocation (Variables|/Script/Engine.Actor|GetRootComponent _array_element) "1.000000,0.000000,0.000000" false false))
  (Development|PrintText (Utilities|Text|FormatText "We have raised {count} Trees." (Utilities|Array|Length _outactors)))
  (Utilities|FlowControl|Delay 3e+01)
  (CallFunction|MakeTreesMove))

(event EventBeginPlay
  ;[0.15 0.15 0.15 0.5] Comment
  (Utilities|FlowControl|Sequence
    (:then_1
      (Utilities|FlowControl|Delay 1.0)
      (CallFunction|MakeTreesMove))))

(fn ConstructionScript)