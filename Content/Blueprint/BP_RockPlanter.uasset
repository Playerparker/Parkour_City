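; BP_RockPlanter is a carryable planter item that the third-person character uses to spawn BP_Tree actors, despite its rock-themed name and debug text.
; On overlap it caches the character and passes itself to PickUpItem.
; Pickup snaps it to the character mesh's hand_r socket, and Drop detaches it.
; PlantSeed spawns a tree at the planter's own transform, adjusting for collisions but always spawning.
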(event Collision|EventActorBeginOverlap
  (params (OtherActor :type Actor%20Object%20Reference))
  (bind _asbp_third_person_character (Utilities|Casting|CastToBP_ThirdPersonCharacter OtherActor))
  (Variables|Default|SetPayer _asbp_third_person_character)
  (Default|PickUpItem _asbp_third_person_character self))

(event EventDrop
  (Transformation|DetachFromActor "KeepRelative" "KeepRelative" "KeepRelative"))

(event EventPlantSeed
  (Development|PrintText "Planting Rocks")
  (Game|SpawnActorfromClass "/Game/Blueprint/BP_Tree.BP_Tree_C" (Transformation|GetActorTransform) "AdjustIfPossibleButAlwaysSpawn" "MultiplyWithRoot" 0 0))

(event EventPickup
  (Development|PrintText "Planter Picked Up")
  (Transformation|AttachComponentToComponent (Variables|/Script/Engine.Character|GetMesh (Variables|Default|GetPayer)) "hand_r" "SnapToTarget" "SnapToTarget" "KeepRelative" true))

(fn ConstructionScript)