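; BP_Tree is a tree actor that grows in stages from BeginPlay, then produces a single fruit.
; A delayed loop enlarges the mesh by random amounts until GrowCounter runs out, then GrowFruit spawns a fruit at FruitSpawn.
; The FruitGrow timeline scales the fruit up and triggers FruitFall, which only sets FruitSpawn to a fixed relative location.
; The physics-based drop logic is disconnected and never runs.
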(event Custom|GrowFruit
  (Development|PrintText "Growing Fruit")
  (bind _returnvalue (Game|SpawnActorfromClass "/Game/Blueprint/BP_Fruit.BP_Fruit_C" (Transformation|GetWorldTransform (Variables|Default|GetFruit%20spawn)) "Undefined" "MultiplyWithRoot" 0 0))
  (bind _newtrack_0 (Timeline|FruitGrow Play)
    (:Update
      (Transformation|SetActorScale3D _returnvalue (Math|Vector|Lerp(Vector) "0.100000,0.100000,0.100000" "1.000000,1.000000,1.000000" _newtrack_0))
      (Timeline|Fruit%20Fall Play
        (:Update
          (Transformation|SetRelativeLocation (Variables|Default|GetFruit%20spawn) "0.000000,0.000000,-1.000000" false false))))))

(event EventBeginPlay
  (bind _staticmesh (Variables|Default|GetStaticMesh))
  (if (> (Variables|Default|GetGrowCounter) 0) :!label _label
    ;[0.15 0.15 0.15 0.5] Comment
    (Utilities|FlowControl|Delay (Math|Random|RandomFloatinRange 4.0 6.0))
    (Transformation|SetRelativeScale3D _staticmesh (+ (Variables|/Script/Engine.SceneComponent|GetRelativeScale3D _staticmesh) (Math|Random|RandomFloatinRange 0.2 0.4)))
    (Math|Integer|DecrementInt (Variables|Default|GetGrowCounter) ; -1 to GC
      (:%20%20
        (goto _label)))
    (else
      (CallFunction|GrowFruit))))

(fn ConstructionScript)